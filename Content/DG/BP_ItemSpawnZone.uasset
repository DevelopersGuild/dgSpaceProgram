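; BP_ItemSpawnZone is a zone actor that periodically spawns random items inside its Box volume.
; BeginPlay starts a looping SpawnTime timer that calls SpawnItems, which does nothing unless IsSpawning is true.
; Each call spawns one random ItemsToSpawn class at a random point in the box, ignoring collisions.
; The random index subtracts one from a zero-to-Length roll, so it can land on -1.
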(event `self.ReceiveBeginPlay`
  (`KismetSystemLibrary.K2_SetTimerDelegate` (delegate `SpawnEvent`) (`self.SpawnTime`) true))

(event `SpawnEvent`
  (`self.SpawnItems`))

(fn `SpawnItems`
  (bind _box (`self.Box`))
  (if (`self.isSpawning`)
    (`|SpawnActorFromClass` (`KismetArrayLibrary.Array_Get` (`self.ItemsToSpawn`) (- (`KismetMathLibrary.RandomIntegerInRange` 0 (`KismetArrayLibrary.Array_Length` (`self.ItemsToSpawn`))) 1)) (`KismetMathLibrary.Conv_VectorToTransform` (`KismetMathLibrary.RandomPointInBoundingBox` (`SceneComponent.K2_GetComponentLocation` _box) (`BoxComponent.BoxExtent` _box))) "AlwaysSpawn" "OverrideRootScale")))

(fn `UserConstructionScript`)